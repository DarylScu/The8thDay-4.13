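; Ceiling light prop for the horror game, built around a point light and a spark burst component.
; The construction script applies the Brightness and Color0 variables to the point light and forces its source radius to zero, leaving the SourceRadius variable unused.
; The event graph has no live runtime logic: Tick is empty and the spark visibility toggles are disconnected.
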(event EventTick
  (params (DeltaSeconds :type Float%20%28single-precision%29)))

(fn ConstructionScript
  (bind _pointlight1 (Variables|Default|GetPointLight1))
  (Utilities|FlowControl|Sequence
    (:then_0
      (Rendering|Components|Light|SetIntensity _pointlight1 (Variables|Light|GetBrightness))
      (Rendering|Components|Light|SetLightColor _pointlight1 (Variables|Light|GetColor_0) true)
      (Class|PointLightComponent|SetSourceRadius _pointlight1 0.0))))