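; Interactable drawer that slides open and spawns a battery.
; A box overlap toggles player input and a gate, so Interact works only while something overlaps the box.
; A FlipFlop, with only its A branch wired, plays a timeline that lerps the mesh from start to end position.
; When the timeline finishes, a short delay precedes spawning Battery_Blueprint at Empymesh's location; a locked-door sound node is left unconnected.
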(event OnComponentBeginOverlap(Box)
  (params (OverlappedComponent :type Primitive%20Component%20Object%20Reference) (OtherActor :type Actor%20Object%20Reference) (OtherComp :type Primitive%20Component%20Object%20Reference) (OtherBodyIndex :type Integer) (bFromSweep :type Boolean) (SweepResult :type Hit%20Result%20Structure%20%28by%20ref%29))
  (Input|EnableInput (Game|GetPlayerController 0))
  (Utilities|FlowControl|Gate true) ; enters at Open
)

(event OnComponentEndOverlap(Box)
  (params (OverlappedComponent :type Primitive%20Component%20Object%20Reference) (OtherActor :type Actor%20Object%20Reference) (OtherComp :type Primitive%20Component%20Object%20Reference) (OtherBodyIndex :type Integer))
  (Input|DisableInput (Game|GetPlayerController 0))
  (Utilities|FlowControl|Gate true) ; enters at Close
)

(event Input|ActionEvents|InputActionInteract
  (params (Key :type Key%20Structure :default "AnyKey"))
  (:Pressed
    (Utilities|FlowControl|Gate true
      (:Exit
        (Utilities|FlowControl|FlipFlop
          (:A
            (bind _driver (Timeline|Timeline_0 Play)
              (:Update
                (Transformation|SetRelativeLocation (Variables|Default|GetStaticMesh) (Math|Vector|Lerp(Vector) (Variables|Default|GetDrawerstart) (Variables|Default|GetDrawerend) _driver) false false))
              (:Finished
                (Utilities|FlowControl|Delay 2.0)
                (Game|SpawnActorfromClass "/Game/HorrorKitDevolpment/Blueprints/Objects/Battery_Blueprint.Battery_Blueprint_C" (Math|Conversions|ToTransform(Vector) (Transformation|GetWorldLocation (Variables|Default|Getempymesh))) "AlwaysSpawn" 0 0)))))))))

(fn ConstructionScript)